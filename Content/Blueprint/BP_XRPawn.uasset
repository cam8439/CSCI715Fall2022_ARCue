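; XR pawn for Magic Leap that nudges a referenced dragon marker actor around the world using touchpad gestures.
; Swipe directions map to X and Y, rotation gestures to Z, and TransformDragonMarker offsets the marker by a fixed step along that axis.
; BeginPlay caches a TextRenderActor, but the audio volume readout, sync threshold check and Lumin camera re-centring logic are disconnected and never run.
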(event OnAudioEnvelopeValue(AudioCapture)
  (params (EnvelopeValue :type Float%20%28single-precision%29)))

(event OnTouchpadGestureStart(MagicLeapTouchpadGestures)
  (params (GestureData :type Magic%20Leap%20Touchpad%20Gesture%20Structure%20%28by%20ref%29))
  (switch Utilities|FlowControl|Switch|SwitchonEMagicLeapTouchpadGestureDirection (.Direction (Utilities|Struct|BreakMagicLeapTouchpadGesture GestureData))
    (:Up
      (CallFunction|TransformDragonMarker "1.000000, 0, 0"))
    (:Down
      (CallFunction|TransformDragonMarker "-1.000000, 0, 0"))
    (:Left
      (CallFunction|TransformDragonMarker "0,-1.000000, 0"))
    (:Right
      (CallFunction|TransformDragonMarker "0,1.000000, 0"))
    (:Clockwise
      (CallFunction|TransformDragonMarker "0,0.000000,1.000000"))
    (:CounterClockwise
      (CallFunction|TransformDragonMarker "0,0.000000,-1.000000"))))

(event EventBeginPlay
  (bind _returnvalue (Actor|GetActorOfClass "/Script/Engine.TextRenderActor"))
  (Variables|Default|SetTextOutput _returnvalue))

(event Collision|EventActorBeginOverlap
  (params (OtherActor :type Actor%20Object%20Reference)))

(event EventTick
  (params (DeltaSeconds :type Float%20%28single-precision%29)))

(event Input|ActionEvents|InputActionMLBumper
  (params (Key :type Key%20Structure)))

(event Input|ActionEvents|InputActionMLTrigger
  (params (Key :type Key%20Structure)))

(fn ConstructionScript)

(fn TransformDragonMarker
  (params (TransformDirection :type Vector))
  (Transformation|SetActorLocation (Variables|Default|GetDragonMarkerRef) (+ (* TransformDirection 2e+01) (Transformation|GetActorLocation (Variables|Default|GetDragonMarkerRef))) false false))