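; Game manager that starts the dragon's movement sequence once the Magic Leap image origin and network are both ready.
; Tick polls CoordinateSyncRef.OriginFound and NetworkReady, clears the network flag, then plays DragonMovementRef's sequence player.
; It binds OnFinished after each play, which calls CallRestart when the sequence ends.
; Image tracker events are empty, and logic to spawn a DragonMarker at the image origin is disconnected.
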(event OnImageTargetFound(MagicLeapImageTracker))

(event OnImageTargetLost(MagicLeapImageTracker))

(event Custom|OnFinished_Event_0
  ;[1 1 1] Try read from the server after playing the sequence
  (Default|CallRestart))

(event Collision|EventActorBeginOverlap
  (params (OtherActor :type Actor%20Object%20Reference)))

(event EventTick
  (params (DeltaSeconds :type Float%20%28single-precision%29))
  (bind _dragonmovementref (Variables|Default|GetDragonMovementRef))
  (bind _sequenceplayer (Variables|/Script/LevelSequence.LevelSequenceActor|GetSequencePlayer _dragonmovementref))
  (if (and (Variables|/Game/Blueprint/CoordinateSync.CoordinateSync_C|GetOriginFound (Variables|Default|GetCoordinateSyncRef)) (Variables|Default|GetNetworkReady))
    (Development|PrintString "Everything is ready" false true "(R=0.000000,G=0.660000,B=1.000000,A=1.000000)" 2e+01)
    (Variables|Default|SetNetworkReady false) ; Reset network status
    (Sequencer|Player|Play _sequenceplayer :!class /Script/MovieScene.MovieSceneSequencePlayer) ; Start Dragon Sequence when Image Found and network is ready
    ;[1 1 1] Try read from the server after playing the sequence
    (EventDispatchers|AssignOnFinished _sequenceplayer (delegate Custom|OnFinished_Event_0))))

(fn ConstructionScript)